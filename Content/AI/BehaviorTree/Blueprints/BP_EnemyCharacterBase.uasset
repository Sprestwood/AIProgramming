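; BP_EnemyCharacterBase is a base enemy character with health, damage-driven death and a floating health bar.
; Construction fills health to max; BeginPlay seeds the WBP_AIHealth widget and caches the first-person player.
; AnyDamage lowers health, updates the widget and destroys the actor at zero, while Tick shows the bar only when the player is within visibility range.
; A helper function sets the movement component's max fly speed.
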(event EventBeginPlay
  (bind _aswbp_aihealth (Utilities|Casting|CastToWBP_AIHealth (UserInterface|GetUserWidgetObject (Variables|Default|GetHealthBar))))
  (Variables|/Game/AI/Widgets/WBP_AIHealth.WBP_AIHealth_C|SetMaxHealth _aswbp_aihealth (Variables|Default|GetEnemyMaxHealth))
  (Variables|Default|SetHealthWidgetRef _aswbp_aihealth)
  (bind _asbp_first_person_character (Utilities|Casting|CastToBP_FirstPersonCharacter (Game|GetPlayerCharacter 0)))
  (Variables|Default|SetPlayerRef _asbp_first_person_character))

(event Game|Damage|EventAnyDamage
  (params (Damage :type Float%20%28single-precision%29) (DamageType :type Damage%20Type%20Object%20Reference) (InstigatedBy :type Controller%20Object%20Reference) (DamageCauser :type Actor%20Object%20Reference))
  (bind _output_get (Variables|Default|SetEnemyHealth (- (Variables|Default|GetEnemyHealth) Damage)))
  (Variables|/Game/AI/Widgets/WBP_AIHealth.WBP_AIHealth_C|SetHealth (Variables|Default|GetHealthWidgetRef) _output_get)
  (if (<= _output_get 0.0)
    (Variables|Default|SetbIsDead true)
    (Actor|DestroyActor)))

(event EventTick
  (params (DeltaSeconds :type Float%20%28single-precision%29))
  (if (<= (Transformation|GetDistanceTo (Variables|Default|GetPlayerRef)) (Variables|Default|GetVisibilityRange))
    (Rendering|SetVisibility (Variables|Default|GetHealthBar) true false)
    (else
      (Rendering|SetVisibility (Variables|Default|GetHealthBar) false false))))

(fn ConstructionScript
  (Variables|Default|SetEnemyHealth (Variables|Default|GetEnemyMaxHealth)))

(fn UpdateFlySpeed
  (params (NewFlySpeed :type Float%20%28double-precision%29))
  (Variables|/Script/Engine.CharacterMovementComponent|SetMaxFlySpeed (Variables|Character|GetCharacterMovement) NewFlySpeed))