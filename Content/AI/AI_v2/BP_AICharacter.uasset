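; BP_AICharacter is an enemy AI with Roam, Patrol and Chase Player states that damages the player at close range.
; AIMoveTo loops drive each state at MaxFlySpeed-based speeds, with PawnSensing or taking damage triggering a chase.
; A distance-gated health bar tracks damage, and death updates player kills plus spawner kills in trials.
; Player death disables sensing and re-runs the current state's behavior.
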(event OnSeePawn(PawnSensing)
  (params (Pawn :type Pawn%20Object%20Reference))
  ;[0 0 0 1 20] Chase Player when AI sees them
  (bind _asbp_first_person_character (Utilities|Casting|CastToBP_FirstPersonCharacter Pawn))
  (CallFunction|ChasePlayer _asbp_first_person_character))

(event Custom|Roam
  ;[0 0 0 1 20] Roam State
  (AI|AIMoveTo self (.RandomLocation (Class|NavigationSystemV1|GetRandomPointinNavigableRadius (Transformation|GetActorLocation) 5e+02 0 0)) 0 5.0 false
    (:OnSuccess
      _)
    (:OnFail
      _))
  (Utilities|FlowControl|Delay 1.0)
  (CallFunction|Roam))

(event Custom|ResetAI
  ;[0 0 0 1 20] Reset AI behavior if Player Died
  (Class|PawnSensingComponent|SetSensingUpdatesEnabled (Variables|Default|GetPawnSensing) false)
  (switch Utilities|FlowControl|Switch|SwitchonE_AIState (Variables|AI|GetAIState)
    (:NewEnumerator1
      (CallFunction|Roam))
    (:NewEnumerator2
      (CallFunction|Patrol))
    (:NewEnumerator3
      (CallFunction|ChasePlayer))))

(event Custom|Patrol
  ;[0 0 0 1 20] Patrol State
  (Variables|/Script/Engine.CharacterMovementComponent|SetMaxFlySpeed (Variables|Character|GetCharacterMovement) (Variables|AI|GetPatrolWalkSpeed))
  (AI|AIMoveTo self "0, 0, 0" (Utilities|Array|Get(acopy) (Variables|AI|GetTargets)) 5.0 false
    (:OnSuccess
      (Utilities|FlowControl|Delay 3.0)
      (AI|AIMoveTo self "0, 0, 0" (Utilities|Array|Get(acopy) (Variables|AI|GetTargets) 1) 5.0 false
        (:OnSuccess
          (Utilities|FlowControl|Delay 3.0)
          (CallFunction|Patrol))))))

(event Custom|ChasePlayer
  (params (PlayerToChase :type Pawn%20Object%20Reference))
  ;[0 0 0 1 20] Chase State
  (if (Variables|/Script/AIModule.PawnSensingComponent|GetbEnableSensingUpdates (Variables|Default|GetPawnSensing))
    (Variables|/Script/Engine.CharacterMovementComponent|SetMaxFlySpeed (Variables|Character|GetCharacterMovement) (Variables|AI|GetChaseSpeed))
    (AI|AIMoveTo self "0, 0, 0" PlayerToChase 5.0 false
      (:OnSuccess
        (if (Utilities|Operators|EqualEqual (Transformation|GetActorLocation) (Transformation|GetActorLocation PlayerToChase) 5e+02)
          (Game|Damage|ApplyDamage PlayerToChase (Variables|AI|GetDamage) 0 0)
          (Utilities|FlowControl|Delay 1.0)
          (CallFunction|ChasePlayer PlayerToChase)))
      (:OnFail
        (CallFunction|Roam)))))

(event EventBeginPlay
  ;[0 0.5 1] FEATURE - Enemy Spawner Logic
  (bind _returnvalue (Actor|GetActorOfClass "/Game/AI/AI_v2/BP_EnemySpawner.BP_EnemySpawner_C"))
  (Variables|AI|SetEnemySpawner _returnvalue)
  ;[0 0 0 1 20] Set starting state behavior
  (bind _aswbp_aihealth_v_2 (Utilities|Casting|CastToWBP_AIHealth_v2 (UserInterface|GetUserWidgetObject (Variables|Default|GetHealthBar))))
  (bind _output_get (Variables|AI|SetHealthBarWidgetRef _aswbp_aihealth_v_2))
  (Variables|/Game/AI/Widgets/WBP_AIHealth_v2.WBP_AIHealth_v2_C|SetMaxHealth _output_get (Variables|AI|GetMaxHealth))
  (bind _asbp_first_person_character (Utilities|Casting|CastToBP_FirstPersonCharacter (Game|GetPlayerCharacter 0)))
  (bind _output_get_2 (Variables|AI|SetPlayerRef _asbp_first_person_character))
  (EventDispatchers|BindEventtoPlayerDied _output_get_2 (delegate Custom|ResetAI))
  (switch Utilities|FlowControl|Switch|SwitchonE_AIState (Variables|AI|GetAIState)
    (:NewEnumerator0
      (CallFunction|ChasePlayer (Variables|AI|GetPlayerRef) :!label _label))
    (:NewEnumerator1
      (CallFunction|Roam))
    (:NewEnumerator2
      (CallFunction|Patrol))
    (:NewEnumerator3
      (goto _label))))

(event EventTick
  (params (DeltaSeconds :type Float%20%28single-precision%29))
  (bind _healthbar (Variables|Default|GetHealthBar))
  ;[0 0 0 1 20] Set AI Health Bar Visibility based on distance to Player
  (if (<= (Transformation|GetDistanceTo (Variables|AI|GetPlayerRef)) (Variables|AI|GetVisibilityRange))
    (Rendering|SetVisibility _healthbar true false)
    (else
      (Rendering|SetVisibility _healthbar false false))))

(event Game|Damage|EventAnyDamage
  (params (Damage :type Float%20%28single-precision%29) (DamageType :type Damage%20Type%20Object%20Reference) (InstigatedBy :type Controller%20Object%20Reference) (DamageCauser :type Actor%20Object%20Reference))
  (bind _playerref (Variables|AI|GetPlayerRef))
  (bind _enemyspawner (Variables|AI|GetEnemySpawner))
  ;[0 0 0 1 20] Damage AI; If Health is Zero, Destroy AI
  (bind _output_get (Variables|AI|SetCurrentHealth (- (Variables|AI|GetCurrentHealth) Damage)))
  (CallFunction|ChasePlayer (Variables|AI|GetPlayerRef))
  (Variables|/Game/AI/Widgets/WBP_AIHealth_v2.WBP_AIHealth_v2_C|SetHealth (Variables|AI|GetHealthBarWidgetRef) _output_get)
  (if (<= _output_get 0.0)
    (Utilities|FlowControl|Sequence
      (:then_0
        (Math|Integer|IncrementInt (Variables|/Game/FirstPerson/Blueprints/BP_FirstPersonCharacter.BP_FirstPersonCharacter_C|GetEnemiesKilled _playerref)
          (:%20%20
            (if (Variables|/Game/FirstPerson/Blueprints/BP_FirstPersonCharacter.BP_FirstPersonCharacter_C|GetbIsTrial _playerref)
              ;[0 0.5 1] FEATURE - Enemy Spawner Logic
              (Math|Integer|IncrementInt (Variables|/Game/AI/AI_v2/BP_EnemySpawner.BP_EnemySpawner_C|GetEnemiesKilled _enemyspawner)
                (:%20%20
                  (Default|CheckEnemiesKilled _enemyspawner)))))))
      (:then_1
        (Actor|DestroyActor)))))

(fn ConstructionScript
  (Variables|AI|SetBaseWalkSpeed (Variables|/Script/Engine.CharacterMovementComponent|GetMaxFlySpeed (Variables|Character|GetCharacterMovement)))
  (Variables|AI|SetCurrentHealth (Variables|AI|GetMaxHealth)))