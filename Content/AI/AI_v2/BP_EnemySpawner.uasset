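; Enemy spawner that runs waves, growing the enemy total by five each time a wave is cleared.
; A looping one-second timer picks one of three scene spawn points and one of three enemy classes by weighted random checks.
; Each check rolls separately, so odds are skewed and some ticks spawn nothing.
; The timer pauses at the wave total and resumes when CheckEnemiesKilled finds the kill count has reached it.
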(event Custom|SpawnEnemy
  (bind _returnvalue (Math|Random|RandomIntegerinRange 0 100))
  (switch int (Math|Random|RandomIntegerinRange 0 2)
    (:0
      (Variables|Default|SetEnemySpawnLocation (Transformation|GetWorldLocation (Variables|Default|GetScene_EnemySpawnLocation))))
    (:1
      (Variables|Default|SetEnemySpawnLocation (Transformation|GetWorldLocation (Variables|Default|GetScene_EnemySpawnLocation1))))
    (:2
      (Variables|Default|SetEnemySpawnLocation (Transformation|GetWorldLocation (Variables|Default|GetScene_EnemySpawnLocation2)))))
  (if (< _returnvalue 50)
    (AI|SpawnAIFromClass (Utilities|Array|Get(acopy) (Variables|Default|GetEnemiesToSpawn)) 0 (Variables|Default|GetEnemySpawnLocation) "0, 0, 0" false 0)
    (bind _result (Math|Integer|IncrementInt (Variables|Default|GetEnemiesSpawned) :!label _label)
      (:%20%20
        (if (>= _result (Variables|Default|GetTotalEnemiesToSpawn))
          (Utilities|Time|PauseTimerbyHandle (Variables|Default|GetSpawnTimerRef)))))
    (elif (and (>= _returnvalue 50) (< _returnvalue 75))
      (AI|SpawnAIFromClass (Utilities|Array|Get(acopy) (Variables|Default|GetEnemiesToSpawn) 1) 0 (Variables|Default|GetEnemySpawnLocation) "0, 0, 0" false 0)
      (goto _label)
      (elif (>= _returnvalue 75)
        (AI|SpawnAIFromClass (Utilities|Array|Get(acopy) (Variables|Default|GetEnemiesToSpawn) 2) 0 (Variables|Default|GetEnemySpawnLocation) "0, 0, 0" false 0)
        (goto _label)))))

(event Custom|CheckEnemiesKilled
  (if (>= (Variables|Default|GetEnemiesKilled) (Variables|Default|GetTotalEnemiesToSpawn))
    (Variables|Default|SetEnemiesSpawned 0)
    (Variables|Default|SetEnemiesKilled 0)
    (Variables|Default|SetTotalEnemiesToSpawn (+ (Variables|Default|GetTotalEnemiesToSpawn) 5))
    (Utilities|Time|UnpauseTimerbyHandle (Variables|Default|GetSpawnTimerRef))))

(event EventBeginPlay
  (bind _returnvalue (Utilities|Time|SetTimerbyEvent (delegate Custom|SpawnEnemy) 1.0 true))
  (Variables|Default|SetSpawnTimerRef _returnvalue))

(fn ConstructionScript)