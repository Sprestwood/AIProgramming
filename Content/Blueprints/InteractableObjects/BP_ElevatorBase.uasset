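; Base interactable elevator that moves its mesh between a start and end point when the player presses Interact.
; Collision overlap with the first-person character enables or disables the actor's input.
; Interact plays or reverses the Lift timeline based on a NAND of CanControl and InAir.
; Each timeline update re-enables control, flips InAir and lerps the mesh's relative location without sweeping.
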(event OnComponentBeginOverlap(Collision)
  (params (OverlappedComponent :type Primitive%20Component%20Object%20Reference) (OtherActor :type Actor%20Object%20Reference) (OtherComp :type Primitive%20Component%20Object%20Reference) (OtherBodyIndex :type Integer) (bFromSweep :type Boolean) (SweepResult :type Hit%20Result%20Structure%20%28by%20ref%29))
  (Utilities|Casting|CastToBP_FirstPersonCharacter OtherActor)
  (Input|EnableInput (Game|GetPlayerController 0)))

(event OnComponentEndOverlap(Collision)
  (params (OverlappedComponent :type Primitive%20Component%20Object%20Reference) (OtherActor :type Actor%20Object%20Reference) (OtherComp :type Primitive%20Component%20Object%20Reference) (OtherBodyIndex :type Integer))
  (Utilities|Casting|CastToBP_FirstPersonCharacter OtherActor)
  (Input|DisableInput (Game|GetPlayerController 0)))

(event EventBeginPlay)

(event Collision|EventActorBeginOverlap
  (params (OtherActor :type Actor%20Object%20Reference)))

(event EventTick
  (params (DeltaSeconds :type Float%20%28single-precision%29)))

(event Input|ActionEvents|InputActionInteract
  (params (Key :type Key%20Structure))
  (:Pressed
    (if (Math|Boolean|NANDBoolean (Variables|Default|GetbCanControl) (Variables|Default|GetbInAir))
      (Variables|Default|SetbCanControl false)
      (bind _time (Timeline|Lift Play)
        (:Update
          (Variables|Default|SetbCanControl true)
          (if (Variables|Default|GetbInAir)
            (Variables|Default|SetbInAir false)
            (else
              (Variables|Default|SetbInAir true)))
          (Transformation|SetRelativeLocation (Variables|Default|GetMesh) (Math|Vector|Lerp(Vector) (Variables|Default|GetStartingPoint) (Variables|Default|GetEndPoint) _time) false false)))
      (else
        (Variables|Default|SetbCanControl false)
        (Timeline|Lift Reverse)))))

(fn ConstructionScript)